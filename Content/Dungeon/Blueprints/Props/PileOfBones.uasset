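; PileOfBones is a dungeon prop that plays a bone-hit sound when the player character type, TopDownCharacter, overlaps its Box.
; A DoOnce gate resets after a short delay, so repeated overlaps cannot spam the sound at the mesh location.
; The construction script gives the static mesh a random yaw within a half turn to vary placed copies.
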(event `self.ReceiveBeginPlay`)

(event `self.Box.OnComponentBeginOverlap`
  (params (OverlappedComponent :type "PrimitiveComponent Object Reference") (OtherActor :type "Actor Object Reference") (OtherComp :type "PrimitiveComponent Object Reference") (OtherBodyIndex :type Integer) (bFromSweep :type Boolean) (SweepResult :type "HitResult Structure (by ref)"))
  (if (`.bSuccess` (cast `/Game/TopDownBP/Blueprints/TopDownCharacter` OtherActor :!pure true))
    (`/Engine/EditorBlueprintResources/StandardMacros.DoOnce` false :!label _label
      (:`Completed`
        (`GameplayStatics.PlaySoundAtLocation` "/Game/Dungeon/Sounds/Skeleton_Hit_Bone.Skeleton_Hit_Bone" (`SceneComponent.K2_GetComponentLocation` (`self.StaticMesh`)) (struct) 2.0 1.0 0.0 null null null)
        (`KismetSystemLibrary.Delay` 1.0)
        (goto _label :!via `Reset`)))))

(fn `UserConstructionScript`
  (`SceneComponent.K2_SetRelativeRotation` (`self.StaticMesh`) (`KismetMathLibrary.MakeRotator` 0.0 0.0 (`KismetMathLibrary.RandomFloatInRange` 0.0 180.0)) false false))