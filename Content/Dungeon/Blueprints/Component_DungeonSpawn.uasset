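; Actor component for BP_DungeonGen that scatters weighted random actors across the dungeon's room floor tiles, optionally including corridors, on BeginPlay.
; It draws tiles from the dungeon's random stream, re-rolling any too close to the previous spawn only.
; Each SpawnList class gets a weighted roll in turn; the first success spawns with offset and optional random yaw.
; Used tiles leave the pool, and the loop repeats until Quantity is reached.
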(event `self.ReceiveBeginPlay`
  (`self.TriggerSpawnThings`))

(event `TriggerSpawnThings`
  (bind _dungeon (`self.Dungeon`))
  (bind _floortiles (`/Game/Dungeon/Blueprints/BP_DungeonGen.FloorTiles` _dungeon))
  (bind _asbp_dungeon_gen (cast `/Game/Dungeon/Blueprints/BP_DungeonGen` (`self.GetOwner`)))
  (set `self.Dungeon` _asbp_dungeon_gen)
  (if (`self.RoomOnly`)
    (set `self.FloorTiles` _floortiles)
    (else
      (set `self.FloorTiles` _floortiles)
      (`KismetArrayLibrary.Array_Append` (`self.FloorTiles`) (`/Game/Dungeon/Blueprints/BP_DungeonGen.CorridorTiles` _dungeon))))
  (`self.Spawn Items`))

(fn `Spawn Items`
  (locals (ItemsSpawned :type Integer) (FloorIndex :type Integer) (lastLocation :type "Vector Structure" :default (0.0 0.0 0.0)))
  (bind _spawnlist (`self.SpawnList`))
  (bind _dungeon (`self.Dungeon`))
  (bind _returnvalue (* (`KismetMathLibrary.Conv_IntVectorToVector` (`|GetArrayItem` (`self.FloorTiles`) (`local.FloorIndex`))) (`/Game/Dungeon/Blueprints/BP_DungeonGen.Scale` _dungeon)))
  ;[1 1 1] While spawns are less then desired quantity loop spawn logic
  (while (> (`self.Quantity`) (`local.ItemsSpawned`))
    ;[1 1 1] Get random floor tile, test if minimum distance is respected
    (bind _output_get (set `local.FloorIndex` (`KismetMathLibrary.RandomIntegerInRangeFromStream` 0 (`KismetArrayLibrary.Array_LastIndex` (`self.FloorTiles`)) (`/Game/Dungeon/Blueprints/BP_DungeonGen.Stream` (`self.Dungeon`))) :!label _label))
    (if (== (`KismetMathLibrary.MakeVector` (.x (* (`KismetMathLibrary.Conv_IntVectorToVector` (`|GetArrayItem` (`self.FloorTiles`) _output_get)) (`/Game/Dungeon/Blueprints/BP_DungeonGen.Scale` (`self.Dungeon`)))) (.y (* (`KismetMathLibrary.Conv_IntVectorToVector` (`|GetArrayItem` (`self.FloorTiles`) _output_get)) (`/Game/Dungeon/Blueprints/BP_DungeonGen.Scale` (`self.Dungeon`))))) (`KismetMathLibrary.MakeVector` (.x (`local.lastLocation`)) (.y (`local.lastLocation`))) :`ErrorTolerance` (`self.MinDistance`))
      (goto _label)
      (else
        ;[1 1 1] Loop through spawn list, if item spawn is true stop looping
        (bind _keys (`BlueprintMapLibrary.Map_Keys` _spawnlist))
        (for _array_element _keys
          (if (`KismetMathLibrary.RandomBoolWithWeightFromStream` (`BlueprintMapLibrary.Map_Find` _spawnlist _array_element) (`/Game/Dungeon/Blueprints/BP_DungeonGen.Stream` (`self.Dungeon`)))
            (`|ExecutionSequence`
              (:`then_0`
                ;[1 1 1] Spawn actor, save previous location, remove tile from list and increment items spawned.
                (`|SpawnActorFromClass` _array_element (`KismetMathLibrary.MakeTransform` (+ _returnvalue (`Actor.K2_GetActorLocation` _dungeon) (`self.Offset`)) (`KismetMathLibrary.MakeRotator` 0.0 0.0 (`KismetMathLibrary.SelectFloat` (`KismetMathLibrary.RandomFloatInRangeFromStream` -180.0 180.0 (`/Game/Dungeon/Blueprints/BP_DungeonGen.Stream` _dungeon)) 0.0 (`self.RandomRotation`)))) "AdjustIfPossibleButAlwaysSpawn" "OverrideRootScale" null null)
                (set `local.lastLocation` _returnvalue)
                (`KismetArrayLibrary.Array_Remove` (`self.FloorTiles`) (`local.FloorIndex`))
                (`/Engine/EditorBlueprintResources/StandardMacros.IncrementInt` (`local.ItemsSpawned`)))
              (:`then_1`
                (break)))))))))