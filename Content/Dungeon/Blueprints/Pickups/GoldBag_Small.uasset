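; Small gold bag pickup that gives money to the player's TopDownCharacter.
; When the static mesh is overlapped by that character, it adds its Gold value to the character's Money, plays a coin sound at the mesh location and destroys itself.
; The construction script gives the mesh a random yaw for visual variety.
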(event `self.StaticMesh.OnComponentBeginOverlap`
  (params (OverlappedComponent :type "PrimitiveComponent Object Reference") (OtherActor :type "Actor Object Reference") (OtherComp :type "PrimitiveComponent Object Reference") (OtherBodyIndex :type Integer) (bFromSweep :type Boolean) (SweepResult :type "HitResult Structure (by ref)"))
  (bind _astop_down_character (cast `/Game/TopDownBP/Blueprints/TopDownCharacter` OtherActor))
  (set `/Game/TopDownBP/Blueprints/TopDownCharacter.Money` (+ (`self.Gold`) (`/Game/TopDownBP/Blueprints/TopDownCharacter.Money` _astop_down_character)) _astop_down_character)
  (`GameplayStatics.PlaySoundAtLocation` "/Game/Dungeon/Sounds/Coins_falling_sound_effect.Coins_falling_sound_effect" (`SceneComponent.K2_GetComponentLocation` (`self.StaticMesh`)) (struct) 1.0 1.0 0.0 null null null)
  (`self.K2_DestroyActor`))

(fn `UserConstructionScript`
  (`SceneComponent.K2_SetWorldRotation` (`self.StaticMesh`) (`KismetMathLibrary.MakeRotator` 0.0 0.0 (`KismetMathLibrary.RandomFloatInRange` 0.0 360.0)) false false))