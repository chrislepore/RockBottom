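; Explosive barrel actor that catches fire when damaged, then explodes and destroys itself.
; Any damage activates fire effect and sound, then after a two-second delay swaps them for an explosion effect and sound.
; The blast applies radial damage twice from the barrel's location, the second call instigated by the player controller, intended to hurt both player and enemies.
; Nothing guards against repeated damage events during the fuse.
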(event `self.ReceiveAnyDamage`
  (params (Damage :type "Float (single-precision)") (DamageType :type "DamageType Object Reference") (InstigatedBy :type "Controller Object Reference") (DamageCauser :type "Actor Object Reference"))
  ;[1 1 1] play fire effect/sound
  (`ActorComponent.Activate` (`self.fire`) false)
  (`ActorComponent.Activate` (`self.fire sound`) false)
  (`KismetSystemLibrary.Delay` 2.0)
  ;[1 1 1] stop fire effect/sound and activate explosion effect
  (`ActorComponent.Deactivate` (`self.fire`))
  (`ActorComponent.Deactivate` (`self.fire sound`))
  (`ActorComponent.Activate` (`self.P_Explosion`) false)
  ;[1 1 1] does damage to player and enemy
  (`GameplayStatics.ApplyRadialDamage` :`BaseDamage` 30.0 :`Origin` (`self.K2_GetActorLocation`) :`DamageRadius` 300.0 :`DamageCauser` self :`InstigatedByController` null :`DamagePreventionChannel` "ECC_WorldStatic")
  (`GameplayStatics.ApplyRadialDamage` :`BaseDamage` 30.0 :`Origin` (`self.K2_GetActorLocation`) :`DamageRadius` 300.0 :`DamageCauser` self :`InstigatedByController` (`GameplayStatics.GetPlayerController` 0) :`DamagePreventionChannel` "ECC_WorldStatic")
  ;[1 1 1] play explosion sound and kill actor
  (`GameplayStatics.PlaySoundAtLocation` "/Game/Weapons/MilitaryWeapDark/Sound/RocketLauncher/RocketLauncher_Explosion_Cue.RocketLauncher_Explosion_Cue" (`self.K2_GetActorLocation`) (struct) 0.5 1.0 0.0 null null null)
  (`KismetSystemLibrary.Delay` 0.2)
  (`self.K2_DestroyActor`))

(fn `UserConstructionScript`)