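; Base projectile actor that deals radial damage when its mesh hits something, then destroys itself.
; On BeginPlay it adds a rocket ammo component and stores it as Ammo, which supplies the damage amount, radius and type.
; Damage is applied in full at the hit location and credited to the instigating controller.
; PlayImpactEffects runs before destruction but is an empty stub, as is the uncalled PlayFireSound.
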(event `self.ReceiveBeginPlay`
  (bind _returnvalue (`AddComponent|NODE_AddBP_AmmoRocket-0`))
  (set `self.Ammo` _returnvalue))

(event `self.Mesh.OnComponentHit`
  (params (HitComponent :type "PrimitiveComponent Object Reference") (OtherActor :type "Actor Object Reference") (OtherComp :type "PrimitiveComponent Object Reference") (NormalImpulse :type "Vector Structure") (Hit :type "HitResult Structure (by ref)"))
  (bind _ammo (`self.Ammo`))
  (`GameplayStatics.ApplyRadialDamage` :`BaseDamage` (`/Game/Weapons/Blueprints/Ammo/BP_AmmoBase.DamageAmount` _ammo) :`Origin` (`.Location` (`GameplayStatics.BreakHitResult` Hit)) :`DamageRadius` (`/Game/Weapons/Blueprints/Ammo/BP_AmmoBase.Radius` _ammo) :`DamageTypeClass` (`/Game/Weapons/Blueprints/Ammo/BP_AmmoBase.DamageType` _ammo) :`DamageCauser` self :`InstigatedByController` (`self.GetInstigatorController`) :`bDoFullDamage` true)
  (`self.Play Impact Effects`)
  (`self.K2_DestroyActor`))

(fn `Play Fire Sound`)

(fn `Play Impact Effects`)

(fn `UserConstructionScript`)