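; Projectile weapon Blueprint that fires spawned projectile actors, with a rocket ammo component added at construction and the ammo count filled to its maximum.
; On fire, a parent-class check either leads to ammo decrement, animation/FX and projectile spawn, or plays the no-ammo sound.
; Projectiles spawn at the muzzle socket along the mesh's forward vector, with a 90-degree correction for the gun's Y axis.
; The fire sound override is empty.
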(event `self.ReceiveBeginPlay`
  (`parent.ReceiveBeginPlay`))

(event `self.OnFire`
  (params (CrosshairWorldspace :type "Vector Structure"))
  (bind _canfire (`self.CanWeaponFire`))
  (if _canfire
    (`self.DecrementAmmoCount`)
    (`self.PlayAnimationAndFX`)
    (`self.PlayFireSound`)
    (`self.FireProjectile`)
    (else
      (`self.PlayNoAmmoSound`))))

(fn `CanWeaponFire`
  (returns (CanFire :type Boolean))
  (bind _canfire (`parent.CanWeaponFire`))
  (return _canfire))

(fn `DecrementAmmoCount`
  (`parent.DecrementAmmoCount`))

(fn `FireProjectile`
  (bind _mesh (`self.Mesh`))
  (`|SpawnActorFromClass` (`self.Projectile`) (`KismetMathLibrary.MakeTransform` (`SceneComponent.GetSocketLocation` _mesh (`self.MuzzleSocket`)) (`KismetMathLibrary.ComposeRotators` (`KismetMathLibrary.Conv_VectorToRotator` (`SceneComponent.GetForwardVector` _mesh)) (struct :`Yaw` 90.0)) (`self.Scale`)) "AlwaysSpawn" "OverrideRootScale" self (`self.GetInstigator`)))

(fn `PlayAnimationAndFX`
  (`parent.PlayAnimationAndFX`))

(fn `PlayFireSound`)

(fn `PlayNoAmmoSound`
  (`parent.PlayNoAmmoSound`))

(fn `UserConstructionScript`
  (`parent.UserConstructionScript`)
  (bind _returnvalue (`AddComponent|NODE_AddBP_AmmoRocket-1`))
  (set `self.Ammo` _returnvalue)
  (set `self.AmmoCount` (`self.AmmoCountMax`)))