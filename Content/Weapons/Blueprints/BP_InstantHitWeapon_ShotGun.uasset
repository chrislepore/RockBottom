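; Shotgun weapon Blueprint, a child class that by its name derives from an instant-hit weapon base.
; The construction script runs the parent's setup, adds a shotgun ammo component as the weapon's Ammo and fills AmmoCount to its maximum.
; BeginPlay and OnFire only forward to the parent, so all firing behavior is inherited.
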(event `self.ReceiveBeginPlay`
  (`parent.ReceiveBeginPlay`))

(event `self.OnFire`
  (params (CrosshairWorldspace :type "Vector Structure"))
  (`parent.OnFire` CrosshairWorldspace))

(fn `UserConstructionScript`
  (`parent.UserConstructionScript`)
  (bind _returnvalue (`AddComponent|NODE_AddBP_AmmoShotgun-1`))
  (set `self.Ammo` _returnvalue)
  (set `self.AmmoCount` (`self.AmmoCountMax`)))