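; Base weapon Blueprint that handles firing, ammo counting and reloading, with an ammo component added at construction.
; OnFire checks ammo and busy flags, decrements ammo and plays the fire animation, whose length sets the firing lockout; an empty weapon clicks at the muzzle.
; Reload plays a montage on the passed AnimInstance alongside the weapon's animation, guarded by a DoOnce, and refills ammo after the montage's duration.
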(event `self.ReceiveBeginPlay`
  (`SkeletalMeshComponent.SetAnimation` (`self.Mesh`) (`self.WeaponReloadAnim`)))

(event `OnFire`
  (params (CrosshairWorldspace :type "Vector Structure"))
  (bind _canfire (`self.CanWeaponFire`))
  (if _canfire
    (set `self.isFiring` true)
    (`self.DecrementAmmoCount`)
    (bind _delaylength (`self.PlayAnimationAndFX`))
    (`KismetSystemLibrary.Delay` _delaylength)
    (set `self.isFiring` false)
    (elif (== (`self.AmmoCount`) 0)
      (`self.PlayNoAmmoSound`))))

(event `Reload`
  (params (`Anim Instance` :type "AnimInstance Object Reference"))
  ;[1 1 1] Reload Weapon
  (if (!= (`self.AmmoCount`) (`self.AmmoCountMax`))
    (`/Engine/EditorBlueprintResources/StandardMacros.DoOnce` false :!label _label
      (:`Completed`
        (set `self.isReloading` true)
        (bind _returnvalue (`AnimInstance.Montage_Play` `Anim Instance` (`self.ReloadWeaponMontage`) 1.0 "MontageLength" 0.0 true))
        (`SkeletalMeshComponent.PlayAnimation` (`self.Mesh`) (`self.WeaponReloadAnim`) false)
        (`KismetSystemLibrary.Delay` _returnvalue)
        (set `self.AmmoCount` (`self.AmmoCountMax`))
        (set `self.isReloading` false)
        (`KismetSystemLibrary.PrintString` "Weapon Reloaded" true false (struct :`G` 1.0 :`A` 1.0))
        (goto _label :!via `Reset`)))))

(fn `CanWeaponFire`
  (returns (CanFire :type Boolean))
  (if (and (> (`self.AmmoCount`) 0) (not (`self.isFiring`)) (not (`self.isReloading`)))
    (return true)
    (else
      (return false))))

(fn `DecrementAmmoCount`
  (bind _output_get (set `self.AmmoCount` (`KismetMathLibrary.Clamp` (- (`self.AmmoCount`) (`self.AmmoPerShot`)) 0 (`self.AmmoCountMax`))))
  (`KismetSystemLibrary.PrintString` (`KismetStringLibrary.BuildString_Int` "" "Ammo: " _output_get)))

(fn `PlayAnimationAndFX`
  (returns (DelayLength :type "Float (double-precision)"))
  (bind _weaponfireanim (`self.WeaponFireAnim`))
  (`SkeletalMeshComponent.PlayAnimation` (`self.Mesh`) _weaponfireanim false)
  (bind _returnvalue (`AnimSequenceBase.GetPlayLength` _weaponfireanim))
  (return _returnvalue))

(fn `PlayNoAmmoSound`
  (`GameplayStatics.PlaySoundAtLocation` "/Game/Weapons/MilitaryWeapDark/CS_No_Ammo_Click_SFX.CS_No_Ammo_Click_SFX" (`SceneComponent.GetSocketLocation` (`self.Mesh`) (`self.MuzzleSocket`)) (struct) 1.0 1.0 0.0 null null null)
  (`KismetSystemLibrary.PrintString` "Out of Ammo" true false (struct :`R` 1.0 :`G` 0.014804 :`A` 1.0)))

(fn `UserConstructionScript`
  (bind _returnvalue (`AddComponent|NODE_AddBP_AmmoBase-1`))
  (set `self.Ammo` _returnvalue)
  (set `self.AmmoCount` (`self.AmmoCountMaxBase`))
  (set `self.FireRate` (`self.FireRateBase`)))