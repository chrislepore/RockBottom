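; Hitscan weapon Blueprint that fires spread line traces from the muzzle and applies point damage to hit actors.
; OnFire checks parent fire and ammo logic, plays effects, and uses a DoOnce reset after FireRate to limit shots.
; DetermineHitObjectsLinear traces random cone directions along muzzle rotation, once per Ammo.Traces, filling HitResults for damage.
; Two crosshair-aimed trace variants are unused here, and PlayImpactEffects is an empty stub.
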(event `self.ReceiveBeginPlay`
  (`parent.ReceiveBeginPlay`))

(event `self.OnFire`
  (params (CrosshairWorldspace :type "Vector Structure"))
  (bind _canfire (`self.CanWeaponFire`))
  (if _canfire
    (`/Engine/EditorBlueprintResources/StandardMacros.DoOnce` false :!label _label
      (:`Completed`
        (set `self.isFiring` true)
        (`self.DecrementAmmoCount`)
        (`self.PlayAnimationAndFX`)
        (bind _hitoccured (`self.DetermineHitObjectsLinear`))
        (if _hitoccured
          (`self.ApplyDamageToHitActors`)
          (`self.PlayImpactEffects`))
        (`KismetSystemLibrary.Delay` (`self.FireRate`))
        (set `self.isFiring` false)
        (goto _label :!via `Reset`)))
    (elif (and (== (`self.AmmoCount`) 0) (not (`self.isReloading`)))
      (`self.PlayNoAmmoSound`))))

(fn `ApplyDamageToHitActors`
  (bind _hitresults (`self.HitResults`))
  (bind _ammo (`self.Ammo`))
  ;[1 1 1] Comment
  (for _index (range (`KismetArrayLibrary.Array_Length` _hitresults))
    (bind _output (`|GetArrayItem` _hitresults _index))
    (bind (_bblockinghit _binitialoverlap _time _distance _location _impactpoint _normal _impactnormal _physmat _hitactor) (`GameplayStatics.BreakHitResult` _output))
    (`GameplayStatics.ApplyPointDamage` _hitactor (`/Game/Weapons/Blueprints/Ammo/BP_AmmoBase.DamageAmount` _ammo) (`KismetMathLibrary.Conv_RotatorToVector` (`KismetMathLibrary.FindLookAtRotation` _location (`self.K2_GetActorLocation` (`Controller.K2_GetPawn` (`self.GetInstigatorController`))))) _output (`self.GetInstigatorController`) self (`/Game/Weapons/Blueprints/Ammo/BP_AmmoBase.DamageType` _ammo))))

(fn `CanWeaponFire`
  (returns (CanFire :type Boolean))
  (bind _canfire (`parent.CanWeaponFire`))
  (return _canfire))

(fn `DecrementAmmoCount`
  (`parent.DecrementAmmoCount`))

(fn `DetermineHitObjectsLinear`
  (returns (HitOccured :type Boolean))
  (locals (ObjectHit :type Boolean))
  (bind (_returnvalue_location _returnvalue_rotation) (`KismetMathLibrary.BreakTransform` (`SceneComponent.GetSocketTransform` (`self.Mesh`) (`self.MuzzleSocket`) "RTS_World")))
  ;[1 1 1] Calculate line trace from muzzel to cursor and add all objects hit to array.
  (`KismetArrayLibrary.Array_Clear` (`self.HitResults`))
  (for _ (range 1 (+ (`/Game/Weapons/Blueprints/Ammo/BP_AmmoBase.Traces` (`self.Ammo`)) 1))
    (bind (_outhit _returnvalue) (`KismetSystemLibrary.LineTraceSingle` _returnvalue_location (+ _returnvalue_location (`KismetMathLibrary.GreaterGreater_VectorRotator` (* (`KismetMathLibrary.RandomUnitVectorInConeInDegrees` (1.0 0.0 0.0) (`self.Spread`)) (`self.Range`)) _returnvalue_rotation)) "TraceTypeQuery1" false (`|MakeArray` (`GameplayStatics.GetPlayerPawn` 0) :!type "Actor Object Reference") "ForDuration"))
    (set `local.ObjectHit` (or _returnvalue (`local.ObjectHit`)))
    (`KismetArrayLibrary.Array_Add` (`self.HitResults`) _outhit))
  (return (`local.ObjectHit`)))

(fn `DeterminHitObjects`
  (params (CrosshairWorldspace :type "Vector Structure"))
  (returns (HitOccured :type Boolean))
  (locals (ObjectHit :type Boolean))
  (bind _returnvalue_location (`KismetMathLibrary.BreakTransform` (`SceneComponent.GetSocketTransform` (`self.Mesh`) (`self.MuzzleSocket`) "RTS_World")))
  (`KismetArrayLibrary.Array_Clear` (`self.HitResults`))
  (for _ (range 1 (+ (`/Game/Weapons/Blueprints/Ammo/BP_AmmoBase.Traces` (`self.Ammo`)) 1))
    (bind (_outhit _returnvalue) (`KismetSystemLibrary.LineTraceSingle` :`Start` _returnvalue_location :`End` (+ _returnvalue_location (`KismetMathLibrary.GreaterGreater_VectorRotator` (* (`KismetMathLibrary.RandomUnitVectorInConeInRadians` (1.0 0.0 0.0) (`KismetMathLibrary.DegreesToRadians` (`self.Spread`))) (`self.Range`)) (`KismetMathLibrary.FindLookAtRotation` _returnvalue_location CrosshairWorldspace))) :`TraceChannel` "TraceTypeQuery1" :`DrawDebugType` "ForDuration"))
    (set `local.ObjectHit` (or _returnvalue (`local.ObjectHit`)))
    (if true
      (`KismetArrayLibrary.Array_Add` (`self.HitResults`) _outhit)))
  (return (`local.ObjectHit`)))

(fn `DeterminHitObjectsPlane`
  (params (CrosshairWorldspace :type "Vector Structure"))
  (returns (HitOccured :type Boolean))
  (locals (ObjectHit :type Boolean))
  (bind (_returnvalue_location _returnvalue_rotation) (`KismetMathLibrary.BreakTransform` (`SceneComponent.GetSocketTransform` (`self.Mesh`) (`self.MuzzleSocket`) "RTS_World")))
  ;[1 1 1] Calculate line trace from muzzel to cursor and add all objects hit to array.
  (`KismetArrayLibrary.Array_Clear` (`self.HitResults`))
  (for _ (range 1 (+ (`/Game/Weapons/Blueprints/Ammo/BP_AmmoBase.Traces` (`self.Ammo`)) 1))
    (bind (_outhit _returnvalue) (`KismetSystemLibrary.LineTraceSingle` :`Start` _returnvalue_location :`End` (+ _returnvalue_location (`KismetMathLibrary.GreaterGreater_VectorRotator` (* (`KismetMathLibrary.RandomUnitVectorInConeInDegrees` (1.0 0.0 0.0) (`self.Spread`)) (`self.Range`)) (`KismetMathLibrary.FindLookAtRotation` _returnvalue_location (`KismetMathLibrary.MakeVector` (.x CrosshairWorldspace) (.y CrosshairWorldspace) (.z _returnvalue_location))))) :`TraceChannel` "TraceTypeQuery1" :`DrawDebugType` "ForDuration"))
    (set `local.ObjectHit` (or _returnvalue (`local.ObjectHit`)))
    (`KismetArrayLibrary.Array_Add` (`self.HitResults`) _outhit))
  (return (`local.ObjectHit`)))

(fn `PlayImpactEffects`)

(fn `UserConstructionScript`
  (`parent.UserConstructionScript`))